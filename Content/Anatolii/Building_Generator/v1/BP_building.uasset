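; Procedural building actor that drives a PCG graph to lay out floors, walls, corners, trims and roof on a modular grid.
; The Construction Script can randomize grid counts and floor count, then derives overall size and height from module dimensions.
; It feeds the resulting offsets, extents and scales into the PCG graph instance as vector parameters, grouped by building part.
; The event graph holds only disabled stubs.
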(event EventBeginPlay)

(event Collision|EventActorBeginOverlap
  (params (OtherActor :type Actor%20Object%20Reference)))

(event EventTick
  (params (DeltaSeconds :type Float%20%28single-precision%29)))

(fn ConstructionScript
  (bind _floor_scale (Variables|Default|GetFloor%20Scale))
  (bind _wallwidth (Variables|Default|GetWallwidth))
  (bind _wallthickness (Variables|Default|GetWallthickness))
  (bind _wallthickness_2 (Variables|Default|GetWallthickness))
  (bind _roof_corner_width (Variables|Default|GetRoof%20corner%20Width))
  (bind _wallwidth_2 (Variables|Default|GetWallwidth))
  (bind _returnvalue (* _wallthickness_2 2.0))
  (bind _returnvalue_2 (* _roof_corner_width 2.0))
  (bind _returnvalue_3 (/ _wallwidth_2 _floor_scale))
  (bind _returnvalue_4 (/ _wallwidth 2.0))
  (Utilities|FlowControl|Sequence
    (:then_0
      ;[0.15 0.15 0.15 0.5] buiding Random
      (if (Variables|Default|GetRandom%20building%20?)
        (Variables|Default|Setbuilding%20Grid%20Count%20X (Math|Random|RandomIntegerinRange 3 10))
        (Variables|Default|Setbuilding%20Grid%20Count%20Y (Math|Random|RandomIntegerinRange 3 8))
        (Variables|Default|SetNumber%20of%20Floors (Math|Random|RandomIntegerinRange 3 5))))
    (:then_1
      (Variables|Default|SetGraph%20Instance (Variables|/Script/PCG.PCGComponent|GetGraphInstance (Variables|Default|GetPCG)))
      (Variables|Default|SetTotal%20Wall%20Size (Math|Vector2D|MakeVector2D (* (Variables|Default|GetWallwidth) (Variables|Default|Getbuilding%20Grid%20Count%20X)) (* (Variables|Default|GetWallwidth) (Variables|Default|Getbuilding%20Grid%20Count%20Y))))
      (bind _output_get (Variables|Default|SetWall%20Half%20Width (/ (Variables|Default|GetWallwidth) 2.0)))
      (Variables|Default|SetNegetive%20Wall%20Half%20Width (* _output_get -1.0))
      (Variables|Default|Setbuilding%20Wall%20Height (+ (* (Variables|Default|GetWallheight) (- (Variables|Default|GetNumber%20of%20Floors) 1)) (Variables|Default|GetTop%20Wall%20Height)))
      (Variables|Default|SetTotal%20building%20Size (Math|Vector2D|MakeVector2D (+ (.x (Variables|Default|GetTotal%20Wall%20Size)) _returnvalue) (+ (.y (Variables|Default|GetTotal%20Wall%20Size)) _returnvalue)))
      (Variables|Default|SetTotal%20building%20Height (+ (Variables|Default|Getbuilding%20Wall%20Height) (Variables|Default|GetRoof%20Trim%20Height) (Variables|Default|GetRoof%20Height))))
    (:then_2
      ;[0.15 0.15 0.15 0.5] Floor
      (Effects|Components|ParticleSystem|SetVectorParameter (Variables|Default|GetGraph%20Instance) "WallGrid_Extent" (Math|Vector|MakeVector (/ (.x (Variables|Default|GetTotal%20Wall%20Size)) 2.0) (/ (.y (Variables|Default|GetTotal%20Wall%20Size)) 2.0) 0.0))
      (Effects|Components|ParticleSystem|SetVectorParameter (Variables|Default|GetGraph%20Instance) "Floor_Scale" (Math|Vector|MakeVector _returnvalue_3 _returnvalue_3 1.0))
      (Effects|Components|ParticleSystem|SetVectorParameter (Variables|Default|GetGraph%20Instance) "Floor_Offset" (Math|Vector|MakeVector (* _returnvalue_4 -1.0) _returnvalue_4 1.0)))
    (:then_3
      ;[0.15 0.15 0.15 0.5] Walls
      (Effects|Components|ParticleSystem|SetVectorParameter (Variables|Default|GetGraph%20Instance) "Wall_offset_1" (Math|Vector|MakeVector 0.0 (Variables|Default|GetWall%20Half%20Width) 0.0))
      (Effects|Components|ParticleSystem|SetVectorParameter (Variables|Default|GetGraph%20Instance) "Wall_offset_2" (Math|Vector|MakeVector 0.0 (Variables|Default|GetNegetive%20Wall%20Half%20Width) 0.0))
      (Effects|Components|ParticleSystem|SetVectorParameter (Variables|Default|GetGraph%20Instance) "Wall_offset_3" (Math|Vector|MakeVector (Variables|Default|GetWall%20Half%20Width) 0.0 0.0))
      (Effects|Components|ParticleSystem|SetVectorParameter (Variables|Default|GetGraph%20Instance) "Wall_offset_4" (Math|Vector|MakeVector (Variables|Default|GetNegetive%20Wall%20Half%20Width) 0.0 0.0))
      (Effects|Components|ParticleSystem|SetVectorParameter (Variables|Default|GetGraph%20Instance) "Wall_offset_adjust" (Math|Vector|MakeVector (Variables|Default|GetNegetive%20Wall%20Half%20Width) (Variables|Default|GetWallthickness) 0.0)))
    (:then_4
      ;[0.15 0.15 0.15 0.5] corner
      (Effects|Components|ParticleSystem|SetVectorParameter (Variables|Default|GetGraph%20Instance) "corner_offset_1" (Math|Vector|MakeVector (Variables|Default|GetNegetive%20Wall%20Half%20Width) (Variables|Default|GetWall%20Half%20Width) 0.0))
      (Effects|Components|ParticleSystem|SetVectorParameter (Variables|Default|GetGraph%20Instance) "corner_offset_2" (Math|Vector|MakeVector (Variables|Default|GetNegetive%20Wall%20Half%20Width) (Variables|Default|GetNegetive%20Wall%20Half%20Width) 0.0))
      (Effects|Components|ParticleSystem|SetVectorParameter (Variables|Default|GetGraph%20Instance) "corner_offset_3" (Math|Vector|MakeVector (Variables|Default|GetWall%20Half%20Width) (Variables|Default|GetNegetive%20Wall%20Half%20Width) 0.0))
      (Effects|Components|ParticleSystem|SetVectorParameter (Variables|Default|GetGraph%20Instance) "corner_offset_4" (Math|Vector|MakeVector (Variables|Default|GetWall%20Half%20Width) (Variables|Default|GetWall%20Half%20Width) 0.0))
      (Effects|Components|ParticleSystem|SetVectorParameter (Variables|Default|GetGraph%20Instance) "Corner_offset_Adjust" (Math|Vector|MakeVector (* _wallthickness -1.0) _wallthickness 0.0)))
    (:then_5
      ;[0.15 0.15 0.15 0.5] Roof corner and bAse
      (Effects|Components|ParticleSystem|SetVectorParameter (Variables|Default|GetGraph%20Instance) "Last_Wall_Point_Adjust" (Math|Vector|MakeVector 0.0 0.0 (Utilities|Operators|Subtract (Variables|Default|Getbuilding%20Wall%20Height) (Variables|Default|GetWallheight) (Variables|Default|GetTop%20Wall%20Height))))
      (Effects|Components|ParticleSystem|SetVectorParameter (Variables|Default|GetGraph%20Instance) "First_Wall_Point_Adjust" (Math|Vector|MakeVector 0.0 0.0 (Variables|Default|GetWallheight)))
      (Effects|Components|ParticleSystem|SetVectorParameter (Variables|Default|GetGraph%20Instance) "Base_trim_Adjust" (Math|Vector|MakeVector 0.0 0.0 (Variables|Default|GetBase%20Wall%20Height%20)))
      (Effects|Components|ParticleSystem|SetVectorParameter (Variables|Default|GetGraph%20Instance) "Roof_Trim_Adjust" (Math|Vector|MakeVector 0.0 0.0 (Variables|Default|Getbuilding%20Wall%20Height)))
      (Effects|Components|ParticleSystem|SetVectorParameter (Variables|Default|GetGraph%20Instance) "Roof_Corner_Adjust" (Math|Vector|MakeVector 0.0 0.0 (+ (Variables|Default|Getbuilding%20Wall%20Height) (Variables|Default|GetRoof%20Trim%20Height))))
      (Effects|Components|ParticleSystem|SetVectorParameter (Variables|Default|GetGraph%20Instance) "Roof_Corner_Pivot_Adjust" (Math|Vector|MakeVector 0.0 (* (Variables|Default|GetRoof%20corner%20Width) -1.0) 0.0)))
    (:then_6
      ;[0.15 0.15 0.15 0.5] Roof horizontal and Vertical
      (Variables|Default|SetBuilding%20Space%20Vertical (- (.x (Variables|Default|GetTotal%20building%20Size)) _returnvalue_2))
      (Variables|Default|SetBuilding%20Space%20Horizontal (- (.y (Variables|Default|GetTotal%20building%20Size)) _returnvalue_2))
      (Effects|Components|ParticleSystem|SetVectorParameter (Variables|Default|GetGraph%20Instance) "Last_roof_Horizontal" (Math|Vector|MakeVector 0.0 (* (- (Variables|Default|GetBuilding%20Space%20Horizontal) (Variables|Default|GetRoof%20Width)) -1.0) 0.0))
      (Effects|Components|ParticleSystem|SetVectorParameter (Variables|Default|GetGraph%20Instance) "Last_roof_Vertical" (Math|Vector|MakeVector 0.0 (* (- (Variables|Default|GetBuilding%20Space%20Vertical) (Variables|Default|GetRoof%20Width)) -1.0) 0.0))
      (Effects|Components|ParticleSystem|SetVectorParameter (Variables|Default|GetGraph%20Instance) "Roof_Top_height_Adjust" (Math|Vector|MakeVector 0.0 0.0 (Variables|Default|GetTotal%20building%20Height)))
      (Effects|Components|ParticleSystem|SetVectorParameter (Variables|Default|GetGraph%20Instance) "Roof_top_Scale_Adjust" (Math|Vector|MakeVector (/ (Variables|Default|GetBuilding%20Space%20Vertical) (Variables|Default|GetRoof%20top%20Size)) (/ (Variables|Default|GetBuilding%20Space%20Horizontal) (Variables|Default|GetRoof%20top%20Size)) 1.0))
      (Effects|Components|ParticleSystem|SetVectorParameter (Variables|Default|GetGraph%20Instance) "Roof_top_Offset_Adjust" (Math|Vector|MakeVector (* (/ (Variables|Default|GetBuilding%20Space%20Vertical) 2.0) -1.0) (/ (Variables|Default|GetBuilding%20Space%20Horizontal) 2.0) 0.0)))
    (:then_7
      (Effects|Components|ParticleSystem|SetVectorParameter (Variables|Default|GetGraph%20Instance) "Top_Floor_Height" (Math|Vector|MakeVector 0.0 0.0 (- (Variables|Default|Getbuilding%20Wall%20Height) (Variables|Default|GetTop%20Wall%20Height)))))))