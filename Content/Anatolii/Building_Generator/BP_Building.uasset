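; BP_Building is a procedural building generator that drives a PCG graph from its construction script.
; When UseAutoRectangle is off, the script rebuilds the spline as a closed, centered Width by Length rectangle.
; In that same branch it derives graph parameters from wall, floor and location values, then calls Generate.
; RoofOffset uses a hardcoded per-floor height rather than WallSize, and the BuildingSize call has no graph instance connected.
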(event EventBeginPlay)

(event Collision|EventActorBeginOverlap
  (params (OtherActor :type Actor%20Object%20Reference)))

(event EventTick
  (params (DeltaSeconds :type Float%20%28single-precision%29)))

(fn ConstructionScript
  (bind _returnvalue (Transformation|GetActorLocation))
  (bind _wall_size (Variables|Default|GetWall%20Size))
  (bind _pcg (Variables|Default|GetPCG))
  (bind _wall_size_2 (Variables|Default|GetWall%20Size))
  (bind _returnvalue_2 (/ _wall_size_2 2.0))
  (bind _returnvalue_3 (/ _wall_size 2.0))
  (bind _graphinstance (Variables|/Script/PCG.PCGComponent|GetGraphInstance _pcg))
  (bind _returnvalue_4 (* _returnvalue_3 -1.0))
  (if (not (Variables|Default|GetUseAutoRectangle))
    (Spline|ClearSplinePoints (Variables|Default|GetSpline) false)
    (Spline|AddSplinePoint (Variables|Default|GetSpline) (Math|Vector|MakeVector (/ (* (Variables|Default|GetWidth) -1.0) 2.0) (/ (* (Variables|Default|GetLength) -1.0) 2.0) 0.0) "Local" false)
    (Spline|AddSplinePoint (Variables|Default|GetSpline) (Math|Vector|MakeVector (/ (* (Variables|Default|GetWidth) 1.0) 2.0) (/ (* (Variables|Default|GetLength) -1.0) 2.0) 0.0) "Local" false)
    (Spline|AddSplinePoint (Variables|Default|GetSpline) (Math|Vector|MakeVector (/ (* (Variables|Default|GetWidth) 1.0) 2.0) (/ (* (Variables|Default|GetLength) 1.0) 2.0) 0.0) "Local" false)
    (Spline|AddSplinePoint (Variables|Default|GetSpline) (Math|Vector|MakeVector (/ (* (Variables|Default|GetWidth) -1.0) 2.0) (/ (* (Variables|Default|GetLength) 1.0) 2.0) 0.0) "Local" false)
    (Spline|SetClosedLoop (Variables|Default|GetSpline) true true)
    (Spline|UpdateSpline (Variables|Default|GetSpline))
    (Effects|Components|ParticleSystem|SetVectorParameter _graphinstance "FloorOffset" (Math|Vector|MakeVector (* _returnvalue_2 -1.0) _returnvalue_2 0.0))
    (Effects|Components|ParticleSystem|SetVectorParameter _graphinstance "FloorScale" (Math|Conversions|ToVector(Float) (/ (Variables|Default|GetFloor%20Size) (Variables|Default|GetWall%20Size))))
    (Effects|Components|ParticleSystem|SetVectorParameter _graphinstance "WallOffset1" (Math|Vector|MakeVector _returnvalue_3 0.0 0.0))
    (Effects|Components|ParticleSystem|SetVectorParameter _graphinstance "WallOffset2" (Math|Vector|MakeVector _returnvalue_4 0.0 0.0))
    (Effects|Components|ParticleSystem|SetVectorParameter _graphinstance "WallOffset3" (Math|Vector|MakeVector 0.0 _returnvalue_3 0.0))
    (Effects|Components|ParticleSystem|SetVectorParameter _graphinstance "WallOffset4" (Math|Vector|MakeVector 0.0 _returnvalue_4 0.0))
    (Effects|Components|ParticleSystem|SetVectorParameter _graphinstance "WallOffsetPivot" (Math|Vector|MakeVector (* (/ (Variables|Default|GetWall%20Size) 2.0) -1.0) (Variables|Default|GetWall%20Thickness) 0.0))
    (Effects|Components|ParticleSystem|SetVectorParameter _graphinstance "BuildingHeight" (Math|Vector|MakeVector 0.0 0.0 (* (Variables|Default|GetWall%20Size) (- (Variables|Default|GetFloors) 1))))
    (Effects|Components|ParticleSystem|SetVectorParameter _graphinstance "FloorCopyOffset" (Math|Vector|MakeVector (* (.z _returnvalue) -1.0) (.y _returnvalue) (* (.x _returnvalue) -1.0)))
    (Effects|Components|ParticleSystem|SetVectorParameter _graphinstance "RoofOffset" (Math|Vector|MakeVector 0.0 0.0 (Math|Conversions|ToFloat(Integer) (* (Variables|Default|GetFloors) 220))))
    (Effects|Components|ParticleSystem|SetVectorParameter 0 "BuildingSize" (Math|Vector|MakeVector (Variables|Default|GetWidth) (Variables|Default|GetLength) 0.0))
    (PCG|Generate (Variables|Default|GetPCG) false)))